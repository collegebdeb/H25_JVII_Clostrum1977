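; Actor component that lets its owner take photos with a scene capture on the Enhanced Input capture action.
; On BeginPlay it adds the photograph mapping context, creates the camera widget and attaches a new SceneCaptureComponent2D to the owner's camera.
; Capturing spawns a BP_Photo attached to the capture component, calls CaptureScene manually and removes the widget.
; A fresh render target is then assigned and stored, so each shot keeps its own texture.
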(event `self.ReceiveBeginPlay`
  (`|ExecutionSequence`
    (:`then_0`
      (`EnhancedInputSubsystemInterface.AddMappingContext` (pcsubsystem `EnhancedInputLocalPlayerSubsystem` (`GameplayStatics.GetPlayerController` 0)) "/Game/Blueprint/Photograph/Inputs/IMC_Photograph.IMC_Photograph" 0 (struct))
      (bind _returnvalue (`|CreateWidget` "/Game/Blueprint/Photograph/UI/UMG_Camera.UMG_Camera_C"))
      (set `self.As UMG_Camera` _returnvalue)
      (bind _returnvalue_2 (`|AddComponentByClass` (`self.GetOwner`) "/Script/Engine.SceneCaptureComponent2D" true (`KismetMathLibrary.MakeTransform` (10.0 0.0 0.0))))
      (set `self.As Scene Capture 2D` _returnvalue_2)
      (`SceneComponent.K2_AttachToComponent` (`self.As Scene Capture 2D`) (`Actor.GetComponentByClass` (`self.GetOwner`) "/Script/Engine.CameraComponent") "None" "KeepRelative" "KeepRelative" "KeepRelative" false)
      (`self.Set Texture Target`))))

(event `EnhancedInput|/Game/Blueprint/Photograph/Inputs/IA_Capture`
  (params (ActionValue :type Boolean) (ElapsedSeconds :type "Float (double-precision)") (TriggeredSeconds :type "Float (double-precision)") (InputAction :type "InputAction Object Reference" :default "/Game/Blueprint/Photograph/Inputs/IA_Capture.IA_Capture"))
  (:`Started`
    (`self.Capture Photo`)
    (`Widget.RemoveFromParent` (`self.As UMG_Camera`))
    (`self.Set Texture Target`)))

(fn `Capture Photo`
  (bind _returnvalue (`|SpawnActorFromClass` "/Game/Blueprint/Photograph/Inputs/BP_Photo.BP_Photo_C" (`KismetMathLibrary.MakeTransform` (1000.0 0.0 0.0) (`KismetMathLibrary.TransformRotation` (`SceneComponent.K2_GetComponentToWorld` (`self.As Scene Capture 2D`)) (struct :`Pitch` 80.0))) "Undefined" "MultiplyWithRoot" null null))
  (bind _output_get (set `self.As BP_Photo` _returnvalue))
  (`Actor.K2_AttachToComponent` _output_get (`self.As Scene Capture 2D`) "None" "KeepRelative" "KeepRelative" "KeepRelative" false)
  (`SceneCaptureComponent2D.CaptureScene` (`self.As Scene Capture 2D`))
  (`KismetSystemLibrary.PrintString` "J'adore les bugs"))

(fn `Set Texture Target`
  (bind _as_scene_capture_2d (`self.As Scene Capture 2D`))
  (bind _returnvalue (`KismetRenderingLibrary.CreateRenderTarget2D` 1920 1080))
  (`KismetArrayLibrary.Array_Add` (`self.Texture Targets`) _returnvalue)
  (set `SceneCaptureComponent2D.TextureTarget` _returnvalue _as_scene_capture_2d)
  (set `SceneCaptureComponent.bCaptureEveryFrame` false _as_scene_capture_2d)
  (set `SceneCaptureComponent.bCaptureOnMovement` false _as_scene_capture_2d)
  (set `SceneCaptureComponent.bAlwaysPersistRenderingState` false _as_scene_capture_2d)
  (set `SceneCaptureComponent2D.FOVAngle` 80.0 _as_scene_capture_2d))