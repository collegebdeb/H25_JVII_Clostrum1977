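; BP_Photo is an actor that displays the player's latest photograph on its Plane mesh.
; When IA_Capture triggers, it reads the last render target in the TextureTargets array of the first-person character's ACPhotograph component.
; It feeds that target into a new dynamic instance of M_Photo, applies it to the Plane and prints a debug string.
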(event `EnhancedInput|/Game/Blueprint/Photograph/Inputs/IA_Capture`
  (params (ActionValue :type Boolean) (ElapsedSeconds :type "Float (double-precision)") (TriggeredSeconds :type "Float (double-precision)") (InputAction :type "InputAction Object Reference" :default "/Game/Blueprint/Photograph/Inputs/IA_Capture.IA_Capture"))
  (:`Triggered`
    (bind _asbp_first_person_character (cast `/Game/FirstPerson/Blueprints/BP_FirstPersonCharacter` (`GameplayStatics.GetPlayerPawn` 0)))
    (bind _returnvalue (`KismetMaterialLibrary.CreateDynamicMaterialInstance` "/Game/Blueprint/Photograph/Inputs/M_Photo.M_Photo"))
    (set `self.Material Instance` _returnvalue)
    (bind _texture_targets (`/Game/Blueprint/Photograph/Inputs/AC_Photograph.Texture Targets` (`/Game/FirstPerson/Blueprints/BP_FirstPersonCharacter.AC_Photograph` _asbp_first_person_character)))
    (`MaterialInstanceDynamic.SetTextureParameterValue` _returnvalue "RenderTarget" (`|GetArrayItem` _texture_targets (- (`KismetArrayLibrary.Array_Length` _texture_targets) 1)))
    (`PrimitiveComponent.SetMaterial` (`self.Plane`) 0 (`self.Material Instance`))
    (`KismetSystemLibrary.PrintString` "ca marche")))

(fn `UserConstructionScript`)