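; Game mode for a local two-player match pitting a first-person Investigator against a third-person Dr. Zurk.
; BeginPlay creates and possesses both characters, randomizing Zurk's start between two PlayerStarts.
; Zurk's spawn branch also scatters evidence across shuffled garden, lab and museum points, plus batteries cycling through shuffled locations.
; Tick counts down match time while the Investigator's HUD shows and isn't paused; reaching zero triggers nothing.
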(event `self.ReceiveTick`
  (params (DeltaSeconds :type "Float (single-precision)"))
  (`self.TempsRestant`)
  (if (== (`self.TempsMonde`) 0.0)
    _))

(event `self.ReceiveBeginPlay`
  (bind _returnvalue (`GameplayStatics.GetPlayerController` 0))
  (bind _outactors (`GameplayStatics.GetAllActorsOfClass` "/Script/Engine.PlayerStart"))
  (bind _output_get (set `self.AllSpawnPoint` _outactors))
  (`KismetArrayLibrary.Array_AddUnique` (`self.AllSpawnPoint_Zurk`) (`|GetArrayItem` _output_get 1))
  (`KismetArrayLibrary.Array_AddUnique` (`self.AllSpawnPoint_Zurk`) (`|GetArrayItem` _output_get 2))
  ; pour chaque Player spawn
  (`KismetArrayLibrary.Array_Shuffle` (`self.AllSpawnPoint_Zurk`))
  (for (_array_element _array_index) (`self.AllSpawnPoint_Zurk`)
    (bind _output_get_2 (set `self.Array Index` _array_index))
    (bind _returnvalue_2 (`GameplayStatics.CreatePlayer` _output_get_2))
    ; Dr.Zurk player
    (if (> (`self.Array Index`) 0)
      (`EnhancedInputSubsystemInterface.AddMappingContext` (pcsubsystem `EnhancedInputLocalPlayerSubsystem` _returnvalue_2) "/Game/ThirdPerson/Input/IMC_Default.IMC_Default" 0 (struct))
      (bind _returnvalue_3 (`|SpawnActorFromClass` "/Game/ThirdPerson/Blueprints/BP_ThirdPersonCharacter.BP_ThirdPersonCharacter_C" (`self.GetTransform` _array_element) "Undefined" "MultiplyWithRoot" null null))
      (`Controller.Possess` (`GameplayStatics.GetPlayerController` (`self.Array Index`)) _returnvalue_3)
      ; apparition de preuve
      (`|ExecutionSequence`
        (:`then_0`
          (bind _outactors_2 (`GameplayStatics.GetAllActorsOfClass` "/Game/Blueprint/BP_SpawnPreuve_Jardin.BP_SpawnPreuve_Jardin_C"))
          (bind _output_get_3 (set `self.Spawn Locations Jardin` _outactors_2))
          (`KismetArrayLibrary.Array_Shuffle` _output_get_3)
          (for _array_element_2 (`self.Spawn Locations Jardin`)
            (`KismetArrayLibrary.Array_Add` (`self.Already Spawned1`) _array_element_2)
            (if (>= (`KismetArrayLibrary.Array_Length` (`self.Already Spawned1`)) (+ (`self.NbrePreuve`) 1))
              (break)
              (else
                (`|SpawnActorFromClass` "/Game/Blueprint/BP_Preuve.BP_Preuve_C" (`self.GetTransform` _array_element_2) "Undefined" "MultiplyWithRoot" null null)
                (`KismetSystemLibrary.PrintString` "Preuve Jardin!" true true (struct :`G` 1.0 :`B` 0.079266 :`A` 1.0))))))
        (:`then_1`
          (bind _outactors_3 (`GameplayStatics.GetAllActorsOfClass` "/Game/Blueprint/BP_SpawnPreuve_Laboratoire.BP_SpawnPreuve_Laboratoire_C"))
          (bind _output_get_4 (set `self.Spawn Location Labo` _outactors_3))
          (`KismetArrayLibrary.Array_Shuffle` _output_get_4)
          (for _array_element_3 (`self.Spawn Location Labo`)
            (`KismetArrayLibrary.Array_Add` (`self.Already Spawned2`) _array_element_3)
            (if (>= (`KismetArrayLibrary.Array_Length` (`self.Already Spawned2`)) (+ (`self.NbrePreuve`) 1))
              (break)
              (else
                (`|SpawnActorFromClass` "/Game/Blueprint/BP_Preuve.BP_Preuve_C" (`self.GetTransform` _array_element_3) "Undefined" "MultiplyWithRoot" null null)
                (`KismetSystemLibrary.PrintString` "Preuve Labo!" true true (struct :`R` 1.0 :`G` 0.033144 :`A` 1.0))))))
        (:`then_2`
          (bind _outactors_4 (`GameplayStatics.GetAllActorsOfClass` "/Game/Blueprint/BP_SpawnPreuve_Muse.BP_SpawnPreuve_Muse_C"))
          (bind _output_get_5 (set `self.Spawn Locations Muse` _outactors_4))
          (`KismetArrayLibrary.Array_Shuffle` _output_get_5)
          (for _array_element_4 (`self.Spawn Locations Muse`)
            (`KismetArrayLibrary.Array_Add` (`self.Already Spawned3`) _array_element_4)
            (if (>= (`KismetArrayLibrary.Array_Length` (`self.Already Spawned3`)) (+ (`self.NbrePreuve`) 1))
              (break)
              (else
                (`|SpawnActorFromClass` "/Game/Blueprint/BP_Preuve.BP_Preuve_C" (`self.GetTransform` _array_element_4) "Undefined" "MultiplyWithRoot" null null)
                (`KismetSystemLibrary.PrintString` "Preuve Muse!" true true (struct :`R` 1.0 :`G` 0.833735 :`A` 1.0))))))
        (:`then_3`
          ; apparition de batteries
          (bind _outactors_5 (`GameplayStatics.GetAllActorsOfClass` "/Game/Blueprint/BP_SpawnBatteries.BP_SpawnBatteries_C"))
          (bind _output_get_6 (set `self.SpawnLocation Batteries` _outactors_5))
          (`KismetArrayLibrary.Array_Shuffle` _output_get_6)
          (for _ (range (`self.NbreBatterie`))
            (`self.SpawnBatterie`)
            (`KismetSystemLibrary.PrintString` "Batterie_Spawned!" true true (struct :`R` 1.0 :`G` 0.783628 :`A` 1.0)))))
      (else
        ; Investigateur Player
        (`EnhancedInputSubsystemInterface.AddMappingContext` (pcsubsystem `EnhancedInputLocalPlayerSubsystem` _returnvalue) "/Game/FirstPerson/Input/IMC_Default.IMC_Default" 0 (struct))
        (bind _returnvalue_4 (`|SpawnActorFromClass` "/Game/FirstPerson/Blueprints/BP_FirstPersonCharacter.BP_FirstPersonCharacter_C" (`self.GetTransform` (`|GetArrayItem` (`self.AllSpawnPoint`))) "Undefined" "MultiplyWithRoot" null false false false false false null null))
        (`Controller.Possess` _returnvalue _returnvalue_4)))))

(fn `SpawnBatterie`
  (bind _output_get (set `self.IndexBatterieLocation` (mod (+ (`self.IndexBatterieLocation`) 1) (`KismetArrayLibrary.Array_Length` (`self.SpawnLocation Batteries`)))))
  (`|SpawnActorFromClass` "/Game/Blueprint/BP_Batteries.BP_Batteries_C" (`self.GetTransform` (`|GetArrayItem` (`self.SpawnLocation Batteries`) _output_get)) "Undefined" "MultiplyWithRoot" null null))

(fn `TempsRestant`
  (bind _asbp_first_person_character (cast `/Game/FirstPerson/Blueprints/BP_FirstPersonCharacter` (`GameplayStatics.GetPlayerCharacter` 0) :!pure true))
  (if (`/Game/FirstPerson/Blueprints/BP_FirstPersonCharacter.surPause?` _asbp_first_person_character)
    (set `self.TempsMonde` (stale _output_get))
    (elif (`/Game/FirstPerson/Blueprints/BP_FirstPersonCharacter.showHUD` _asbp_first_person_character)
      (bind _output_get (set `self.TempsMonde` (`KismetMathLibrary.FClamp` (- (`self.TempsMonde`) (`GameplayStatics.GetWorldDeltaSeconds`)) 0.0 (`self.TempsMonde`)))))))

(fn `UserConstructionScript`)