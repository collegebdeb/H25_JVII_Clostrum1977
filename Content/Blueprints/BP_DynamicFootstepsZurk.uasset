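; Anim notify for Zurk footsteps that shakes the first player's camera according to how close the second player's pawn is.
; Within a range threshold, it starts BP_CameraShake on player controller 0, with intensity mapped inversely from the distance between pawns 0 and 1.
; It also line-traces downward from the mesh owner, but the result is unused and no sound plays here.
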(fn `Received_Notify`
  (params (MeshComp :type "SkeletalMeshComponent Object Reference") (Animation :type "AnimSequenceBase Object Reference") (EventReference :type "AnimNotifyEventReference Structure (by ref)"))
  (returns (ReturnValue :type Boolean))
  (bind _returnvalue (`ActorComponent.GetOwner` MeshComp))
  (bind _returnvalue_2 (`Actor.K2_GetActorLocation` _returnvalue))
  (bind _returnvalue_3 (`Actor.GetDistanceTo` (`GameplayStatics.GetPlayerPawn` 0) (`GameplayStatics.GetPlayerPawn` 1)))
  ; Met en place les points de reperes qui vont inclure les fonctions qu'on attribuera
  (`KismetSystemLibrary.LineTraceSingle` _returnvalue_2 (+ _returnvalue_2 (* (`Actor.GetActorUpVector` _returnvalue) -200.0)) "TraceTypeQuery1")
  (if (<= _returnvalue_3 5000.0)
    ; Jouer le camera shakepour le first person character lorsque le son de pas est joué
    (bind _asplayer_controller (cast `PlayerController` (`GameplayStatics.GetPlayerController` 0)))
    (`PlayerController.ClientStartCameraShake` :`self` _asplayer_controller :`Shake` "/Game/Blueprint/BP_CameraShake.BP_CameraShake_C" :`Scale` (`KismetMathLibrary.MapRangeClamped` _returnvalue_3 1000.0 5000.0 8.0 0.2)))
  (return false))